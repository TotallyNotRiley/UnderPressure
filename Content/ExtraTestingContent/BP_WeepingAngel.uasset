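; BP_WeepingAngel is a test character that chases the player only while its mesh is off screen, in the style of a weeping angel.
; Each tick it checks whether the mesh was recently rendered, rather than tracing line of sight.
; When unseen it uses simple move-to toward player 0 and plays animation normally.
; When rendered while moving, it stops the controller, zeroes velocity and freezes the animation through the global rate scale.
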(event `self.ReceiveTick`
  (params (DeltaSeconds :type "Float (single-precision)"))
  (bind _returnvalue (`self.GetController`))
  (if (`PrimitiveComponent.WasRecentlyRendered` (`self.Mesh`) 0.05)
    (if (`self.IsMoving`)
      (`Controller.StopMovement` _returnvalue)
      (set `self.IsMoving` false)
      (set `SkeletalMeshComponent.GlobalAnimRateScale` 0.0 (`self.Mesh`))
      (set `MovementComponent.Velocity` (0.0 0.0 0.0) (`self.CharacterMovement`)))
    (else
      (`AIBlueprintHelperLibrary.SimpleMoveToLocation` _returnvalue (`self.K2_GetActorLocation` (`GameplayStatics.GetPlayerCharacter` 0)))
      (set `self.IsMoving` true)
      (set `SkeletalMeshComponent.GlobalAnimRateScale` 1.0 (`self.Mesh`)))))

(fn `UserConstructionScript`)